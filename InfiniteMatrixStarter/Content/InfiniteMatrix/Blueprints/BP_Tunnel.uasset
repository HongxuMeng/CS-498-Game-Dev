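; BP_Tunnel is a tunnel segment with a rotating holed wall that the player must get through.
; RandomizeWall picks one of four hole meshes and a random starting roll, and Tick keeps the wall spinning.
; Touching the wall processes a player hit and destroys the segment's health pack and enemy.
; The end trigger awards score if the wall was not hit, asks TunnelSpawner for another tunnel, then destroys the segment and its pickup and enemy.
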(event `self.ReceiveBeginPlay`)

(event `self.ReceiveTick`
  (params (DeltaSeconds :type "Float (single-precision)"))
  (`SceneComponent.K2_AddLocalRotation` (`self.WallMesh`) (`KismetMathLibrary.MakeRotator` (* DeltaSeconds (`self.RotateSpeed`))) false false))

(event `self.TriggerZone.OnComponentBeginOverlap`
  (params (OverlappedComponent :type "PrimitiveComponent Object Reference") (OtherActor :type "Actor Object Reference") (OtherComp :type "PrimitiveComponent Object Reference") (OtherBodyIndex :type Integer) (bFromSweep :type Boolean) (SweepResult :type "HitResult Structure (by ref)"))
  ;[1 1 1] Reach the end of tunnel
  (bind _asbp_player (cast `/Game/InfiniteMatrix/Blueprints/BP_Player` OtherActor))
  (if (not (`self.JustHitWall`))
    (`/Game/InfiniteMatrix/Blueprints/BP_Player.UpdateScore` _asbp_player (`/Game/InfiniteMatrix/Blueprints/BP_Player.ScoreTunnel` _asbp_player)))
  (`/Game/InfiniteMatrix/Blueprints/BP_TunnelSpawner.SpawnTunnelAtSpawnPoint` (`self.TunnelSpawner`))
  (`|ExecutionSequence`
    (:`then_0`
      (`self.DestroyHealthPack`))
    (:`then_1`
      (`self.DestroyEnemy`))
    (:`then_2`
      (`/Engine/EditorBlueprintResources/StandardMacros.IsValid` self
        (:`Is Valid`
          (`self.K2_DestroyActor`))))))

(event `self.WallMesh.OnComponentBeginOverlap`
  (params (OverlappedComponent :type "PrimitiveComponent Object Reference") (OtherActor :type "Actor Object Reference") (OtherComp :type "PrimitiveComponent Object Reference") (OtherBodyIndex :type Integer) (bFromSweep :type Boolean) (SweepResult :type "HitResult Structure (by ref)"))
  ;[1 1 1] Hit on wall
  (bind _asbp_player (cast `/Game/InfiniteMatrix/Blueprints/BP_Player` OtherActor))
  (`/Game/InfiniteMatrix/Blueprints/BP_Player.ProcessHit` _asbp_player)
  (set `self.JustHitWall` true)
  (`self.DestroyHealthPack`)
  (`self.DestroyEnemy`))

(event `self.WallMesh.OnComponentHit`
  (params (HitComponent :type "PrimitiveComponent Object Reference") (OtherActor :type "Actor Object Reference") (OtherComp :type "PrimitiveComponent Object Reference") (NormalImpulse :type "Vector Structure") (Hit :type "HitResult Structure (by ref)"))
  ;[1 1 1] Old from tutorial
)

(fn `DestroyEnemy`
  (bind _tunnelenemy (`self.TunnelEnemy`))
  (`/Engine/EditorBlueprintResources/StandardMacros.IsValid` _tunnelenemy
    (:`Is Valid`
      (`self.K2_DestroyActor` _tunnelenemy))))

(fn `DestroyHealthPack`
  (bind _tunnelhealthpack (`self.TunnelHealthPack`))
  (`/Engine/EditorBlueprintResources/StandardMacros.IsValid` _tunnelhealthpack
    (:`Is Valid`
      (`self.K2_DestroyActor` _tunnelhealthpack))))

(fn `RandomizeWall`
  (`StaticMeshComponent.SetStaticMesh` (`self.WallMesh`) (select `int` (`KismetMathLibrary.RandomIntegerInRange` 0 3) :`0` "/Game/InfiniteMatrix/Meshes/SM_Hole_01.SM_Hole_01" :`1` "/Game/InfiniteMatrix/Meshes/SM_Hole_02.SM_Hole_02" :`2` "/Game/InfiniteMatrix/Meshes/SM_Hole_03.SM_Hole_03" :`3` "/Game/InfiniteMatrix/Meshes/SM_Hole_04.SM_Hole_04" :!type "StaticMesh Object Reference"))
  (`SceneComponent.K2_AddLocalRotation` (`self.WallMesh`) (`KismetMathLibrary.MakeRotator` (`KismetMathLibrary.RandomFloatInRange` 0.0 360.0)) false false))

(fn `UserConstructionScript`)